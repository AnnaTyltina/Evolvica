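; Food pickup actor that raises an Evolvica character's satiety when eaten.
; On construction it picks a random skeletal mesh and rolls a random mutation (eyes, legs or wings) into its monster attributes.
; Overlap by an Evolvica character adds its satiety points, prints a debug message and destroys the food.
; The rolled mutation is only printed at BeginPlay and is not passed to the character.
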(event OnComponentBeginOverlap(FoodCollision)
  (params (OverlappedComponent :type Primitive%20Component%20Object%20Reference) (OtherActor :type Actor%20Object%20Reference) (OtherComp :type Primitive%20Component%20Object%20Reference) (OtherBodyIndex :type Integer) (bFromSweep :type Boolean) (SweepResult :type Hit%20Result%20Structure%20%28by%20ref%29))
  (bind _asevolvica_character (Utilities|Casting|CastToEvolvica_Character OtherActor))
  (Default|IncreaseSatiety _asevolvica_character (Variables|Default|GetSatietyPoints))
  (Development|PrintString "Picked")
  (Actor|DestroyActor))

(event EventBeginPlay
  (Development|PrintString (Utilities|String|EnumtoString (.mutations (Variables|Default|GetMonsterAttributes)))))

(fn ConstructionScript
  (bind _array (Utilities|Array|MakeArray "/Engine/EngineMeshes/SkeletalCube.SkeletalCube" "/Engine/EditorMeshes/SkeletalMesh/DefaultSkeletalMesh.DefaultSkeletalMesh" "/Game/Assets/Meshes/SK_Mannequin.SK_Mannequin"))
  (Class|SkinnedMeshComponent|SetSkeletalMesh (Variables|Default|GetFoodMesh) (Utilities|Array|Get(acopy) _array (Math|Random|RandomIntegerinRange 0 (- (Utilities|Array|Length _array) 1))) true)
  (Variables|Default|SetMonsterAttributes (Utilities|Struct|MakeMonsterAttributes_S 0 (Utilities|Select :Index (Utilities|Enum|ByteToEnumMutations_E (Math|Conversions|ToByte(Integer) (Math|Random|RandomIntegerinRange 0 (|GetNumEnumEntries)))) :NewEnumerator0 "NewEnumerator0" :NewEnumerator1 "NewEnumerator1" :NewEnumerator2 "NewEnumerator2"))))