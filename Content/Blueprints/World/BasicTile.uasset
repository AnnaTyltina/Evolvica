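; Track tile for Evolvica that chains to the next tile and fills itself with a random obstacle, food or nothing.
; On BeginPlay, a random integer is mapped through range checks to a spawn type, slightly favoring empty, and the matching class spawns at SpawnPoint.
; When the character overlaps SpawnTrigger, the tile asks Evolvica_PC to spawn the next tile, then destroys itself after a short delay.
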(event OnComponentBeginOverlap(SpawnTrigger)
  (params (OverlappedComponent :type Primitive%20Component%20Object%20Reference) (OtherActor :type Actor%20Object%20Reference) (OtherComp :type Primitive%20Component%20Object%20Reference) (OtherBodyIndex :type Integer) (bFromSweep :type Boolean) (SweepResult :type Hit%20Result%20Structure%20%28by%20ref%29))
  (Utilities|Casting|CastToEvolvica_Character OtherActor)
  (bind _asevolvica_pc (Utilities|Casting|CastToEvolvica_PC (Game|GetPlayerController 0)))
  (Default|SpawnNextTile _asevolvica_pc)
  (Utilities|FlowControl|Delay 1.5)
  (Actor|DestroyActor))

(event EventBeginPlay
  (CallFunction|ChooseandSpawn))

(fn ConstructionScript)

(fn ChooseandSpawn
  ;[1 1 1] TODO: Rename
  (Variables|Default|SetRandomInteger (Math|Random|RandomIntegerinRange 0 8))
  (bind _index (CallFunction|Choose))
  (CallFunction|Spawn (Utilities|Select :Index _index :NewEnumerator0 0 :NewEnumerator1 "/Game/Blueprints/World/ObstacleSmall_BP.ObstacleSmall_BP_C" :NewEnumerator3 "/Game/Blueprints/World/ObstacleBig_BP.ObstacleBig_BP_C" :NewEnumerator2 "/Game/Blueprints/World/Food_BP.Food_BP_C")))

(fn Spawn
  (params (ToSpawn :type Actor%20Class%20Reference))
  ;[1 1 1] TODO: Rename
  (Game|SpawnActorfromClass ToSpawn (Math|Transform|MakeTransform (Transformation|GetWorldLocation (Variables|Default|GetSpawnPoint)) "0, 0, 0" "1,1,1") "Undefined" 0 0))

(fn IfBelongstoSegment
  (params (Number :type Integer) (Min :type Integer) (Max :type Integer))
  ;[1 1 1] Rename
  (return (and (>= Number Min) (<= Number Max))))

(fn Choose
  (if (CallFunction|IfBelongstoSegment (Variables|Default|GetRandomInteger) 0 2)
    (return "NewEnumerator0")
    (elif (CallFunction|IfBelongstoSegment (Variables|Default|GetRandomInteger) 3 4)
      (return "NewEnumerator1")
      (elif (CallFunction|IfBelongstoSegment (Variables|Default|GetRandomInteger) 5 6)
        (return "NewEnumerator3")
        (elif (CallFunction|IfBelongstoSegment (Variables|Default|GetRandomInteger) 7 8)
          (return "NewEnumerator2"))))))