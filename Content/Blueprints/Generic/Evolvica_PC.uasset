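; Player controller for Evolvica that sets up the on-screen widget and lays down the opening chain of tiles.
; On BeginPlay it creates Screen_W, keeps a reference, adds it to the viewport and spawns a starting batch of tiles.
; SpawnNextTile places each BasicTile at the stored next location, then takes that tile's SpawnPoint position as the following one, so tiles link end to end.
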(event EventBeginPlay
  (bind _returnvalue (UserInterface|CreateWidget "/Game/Blueprints/Widgets/Screen_W.Screen_W_C"))
  (bind _output_get (Variables|Default|SetScreen_Ref _returnvalue))
  (UserInterface|Viewport|AddtoViewport _output_get 0)
  ;[1 1 1] Spawn First Tiles
  (for _index (range 0 4)
    (CallFunction|SpawnNextTile)))

(fn ConstructionScript)

(fn SpawnNextTile
  (bind _returnvalue (Game|SpawnActorfromClass "/Game/Blueprints/World/BasicTile.BasicTile_C" (Variables|Default|GetNextSpawnLocation) "Undefined" 0 0))
  (Variables|Default|SetNextSpawnLocation (Math|Transform|MakeTransform (Transformation|GetWorldLocation (Variables|/Game/Blueprints/World/BasicTile.BasicTile_C|GetSpawnPoint _returnvalue)) "0, 0, 0" "1,1,1")))